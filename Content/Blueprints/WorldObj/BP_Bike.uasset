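; BP_Bike is a self-moving bike world object that also serves as a camera view target.
; Each Tick spins the front and back cubes and applies a velocity-change impulse on +Y to the frame, unscaled by delta time.
; MoveToNextBike blends the first player's camera to a random BP_Bike, which may be itself.
; An unconnected chain would blend the view to BP_Player.
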(event Custom|MoveToNextBike
  (bind _outactors (Actor|GetAllActorsOfClass "BP_Bike_C"))
  (if (Utilities|IsValid (.OutItem (Utilities|Array|Random _outactors)))
    (Game|Player|SetViewTargetwithBlend (Game|GetPlayerController (Game|GetPlayerState 0)) (.OutItem (Utilities|Array|Random _outactors)) 1.0 "VTBlend_Linear" 0.0 false)))

(event EventBeginPlay)

(event Collision|EventActorBeginOverlap
  (params (OtherActor :type Actor%20Object%20Reference)))

(event EventTick
  (params (DeltaSeconds :type Float%20%28single-precision%29))
  (Transformation|AddLocalRotation (Variables|Default|GetBackCube) "0, 0,10.000000" false false)
  (Transformation|AddLocalRotation (Variables|Default|GetFrontCube) "0, 0,10.000000" false false)
  (Physics|AddImpulse (Variables|Default|GetBike_Frame) "0,30.000000, 0" "None" true))

(fn ConstructionScript)