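; BP_Door is a two-way door that swings open when the player walks into a trigger on either side.
; EnterBox and ExitBox overlaps snap DoorFrontDoor 90 degrees in opposite directions, then snap it shut after DoorCloseDelay.
; CheckForDoor uses the enter and exit flags to ignore both triggers while the door is open.
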(event OnComponentBeginOverlap(EnterBox)
  (params (OverlappedComponent :type Primitive%20Component%20Object%20Reference) (OtherActor :type Actor%20Object%20Reference) (OtherComp :type Primitive%20Component%20Object%20Reference) (OtherBodyIndex :type Integer) (bFromSweep :type Boolean) (SweepResult :type Hit%20Result%20Structure%20%28by%20ref%29))
  (Utilities|Casting|CastToBP_Player OtherActor)
  (if (CallFunction|CheckforDoor)
    (Transformation|SetRelativeRotation (Variables|Default|GetDoor_FrontDoor) "0,90.000000, 0" false false)
    (Variables|Default|SetIsEnterEnabled? true)
    (Utilities|FlowControl|Delay (Variables|Default|GetDoorCloseDelay))
    (Transformation|SetRelativeRotation (Variables|Default|GetDoor_FrontDoor) "0,0.000000, 0" false false)
    (Variables|Default|SetIsEnterEnabled? false)))

(event OnComponentBeginOverlap(ExitBox)
  (params (OverlappedComponent :type Primitive%20Component%20Object%20Reference) (OtherActor :type Actor%20Object%20Reference) (OtherComp :type Primitive%20Component%20Object%20Reference) (OtherBodyIndex :type Integer) (bFromSweep :type Boolean) (SweepResult :type Hit%20Result%20Structure%20%28by%20ref%29))
  (Utilities|Casting|CastToBP_Player OtherActor)
  (if (CallFunction|CheckforDoor)
    (Transformation|SetRelativeRotation (Variables|Default|GetDoor_FrontDoor) "0,-90.000000, 0" false false)
    (Variables|Default|SetIsExitEnabled? true)
    (Utilities|FlowControl|Delay (Variables|Default|GetDoorCloseDelay))
    (Transformation|SetRelativeRotation (Variables|Default|GetDoor_FrontDoor) "0,0.000000, 0" false false)
    (Variables|Default|SetIsExitEnabled? false)))

(event EventBeginPlay)

(event Collision|EventActorBeginOverlap
  (params (OtherActor :type Actor%20Object%20Reference)))

(event EventTick
  (params (DeltaSeconds :type Float%20%28single-precision%29)))

(fn ConstructionScript)

(fn CheckforDoor
  (return (and (not (Variables|Default|GetIsExitEnabled?)) (not (Variables|Default|GetIsEnterEnabled?)))))